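; BP_Item is a world pickup that the top-down character collects into its inventory.
; On BeginPlay, it fills an unset ItemObject from GetDefaultItemObject, which returns nothing in this Blueprint.
; When BP_TopDownCharacter overlaps the Sphere, the item passes ItemObject to the character's BPInventoryComponent through TryAddItem and destroys itself only if the add succeeds.
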(event `self.ReceiveBeginPlay`
  (if (not (`KismetSystemLibrary.IsValid` (`self.Item Object`)))
    (bind _itemobject (`self.GetDefaultItemObject`))
    (set `self.Item Object` _itemobject)))

(event `self.Sphere.OnComponentBeginOverlap`
  (params (OverlappedComponent :type "PrimitiveComponent Object Reference") (OtherActor :type "Actor Object Reference") (OtherComp :type "PrimitiveComponent Object Reference") (OtherBodyIndex :type Integer) (bFromSweep :type Boolean) (SweepResult :type "HitResult Structure (by ref)"))
  (bind _asbp_top_down_character (cast `/Game/TopDown/Blueprints/BP_TopDownCharacter` OtherActor))
  (bind _added (`/Game/Inventory/BP_InventoryComponent.TryAddItem` (`/Game/TopDown/Blueprints/BP_TopDownCharacter.BP_InventoryComponent` _asbp_top_down_character) (`self.Item Object`)))
  (if _added
    (`self.K2_DestroyActor`)))

(fn `GetDefaultItemObject`
  (returns (ItemObject :type "/Game/Items/BP_ItemObject Object Reference"))
  (return null))

(fn `UserConstructionScript`)