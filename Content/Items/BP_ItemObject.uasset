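; BP_ItemObject is an item data object exposing an item's grid dimensions, icon, class and gold value through getter functions.
; GetIcon returns either the normal or the rotated icon based on the Rotated flag, while GetDimensions returns the stored Dimensions unchanged.
; The other getters return the stored ItemClass and GoldValue directly.
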(fn `GetDimensions`
  (returns (Dimensions :type "IntPoint Structure"))
  (return (`self.Dimensions`)))

(fn `GetIcon`
  (returns (Icon :type "MaterialInterface Object Reference"))
  (return (select `bool` (`self.Rotated`) :`false` (`self.Icon`) :`true` (`self.IconRotated`))))

(fn `GetItemClass`
  (returns (ItemClass :type "/Game/Items/BP_Item Class Reference"))
  (return (`self.ItemClass`)))

(fn `GetValue`
  (returns (Value :type Integer))
  (return (`self.GoldValue`)))